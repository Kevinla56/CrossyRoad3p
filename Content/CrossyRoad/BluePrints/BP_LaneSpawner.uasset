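; Lane spawner for a Crossy Road-style game that builds the initial strip of random terrain lanes on BeginPlay.
; The first lane spawns at a fixed location, each following one at the newest lane's SpawnPoint, and every lane receives a reference back to the spawner.
; A random integer switch weights lane types through repeated cases, favoring grass, then road, then river and railroad, though both river spawns have no class set.
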(event EventBeginPlay
  (CallFunction|SpawnInitialLane))

(event Collision|EventActorBeginOverlap
  (params (OtherActor :type Actor%20Object%20Reference)))

(event EventTick
  (params (DeltaSeconds :type Float%20%28single-precision%29)))

(fn ConstructionScript)

(fn SpawnInitialLane
  (for _index (range 0 20)
    (Utilities|IsValid (Variables|Default|GetNewestLane)
      (:Is%20Valid
        (CallFunction|SpawnLaneatSpawnPoint))
      (:Is%20Not%20Valid
        (CallFunction|SpawnLane "1000.000000,0.000000,10.000000")))))

(fn SpawnLane
  (params (SpawnLocation :type Vector))
  (bind _randomlane (CallFunction|SpawnRandomLane SpawnLocation))
  (bind _output_get (Variables|Default|SetNewestLane _randomlane))
  (Variables|/Game/CrossyRoad/BluePrints/BP_Lane.BP_Lane_C|SetLaneSpawner _output_get self))

(fn SpawnLaneatSpawnPoint
  (CallFunction|SpawnLane (Transformation|GetWorldLocation (Variables|/Game/CrossyRoad/BluePrints/BP_Lane.BP_Lane_C|GetSpawnPoint (Variables|Default|GetNewestLane)))))

(fn SpawnRandomLane
  (params (SpawnLocation :type Vector))
  (switch int (Math|Random|RandomIntegerinRange 0 9)
    (:0
      (bind _returnvalue (Game|SpawnActorfromClass "/Game/CrossyRoad/BluePrints/grAsss.grAsss_C" (Math|Transform|MakeTransform SpawnLocation "0, 0, 0" "1.000000,1.000000,1.000000") "Undefined" 0 0))
      (return _returnvalue))
    (:1
      (bind _returnvalue_2 (Game|SpawnActorfromClass "/Game/CrossyRoad/BluePrints/grAsss.grAsss_C" (Math|Transform|MakeTransform SpawnLocation "0, 0, 0" "1.000000,1.000000,1.000000") "Undefined" 0 0))
      (return _returnvalue_2))
    (:2
      (bind _returnvalue_3 (Game|SpawnActorfromClass "/Game/CrossyRoad/BluePrints/grAsss.grAsss_C" (Math|Transform|MakeTransform SpawnLocation "0, 0, 0" "1.000000,1.000000,1.000000") "Undefined" 0 0))
      (return _returnvalue_3))
    (:3
      (bind _returnvalue_4 (Game|SpawnActorfromClass "/Game/CrossyRoad/BluePrints/grAsss.grAsss_C" (Math|Transform|MakeTransform SpawnLocation "0, 0, 0" "1.000000,1.000000,1.000000") "Undefined" 0 0))
      (return _returnvalue_4))
    (:4
      (bind _returnvalue_5 (Game|SpawnActorfromClass "/Game/CrossyRoad/BluePrints/Road.Road_C" (Math|Transform|MakeTransform SpawnLocation "0, 0, 0" "1.000000,1.000000,1.000000") "Undefined" 0 0))
      (return _returnvalue_5))
    (:5
      (bind _returnvalue_6 (Game|SpawnActorfromClass "/Game/CrossyRoad/BluePrints/Road.Road_C" (Math|Transform|MakeTransform SpawnLocation "0, 0, 0" "1.000000,1.000000,1.000000") "Undefined" 0 0))
      (return _returnvalue_6))
    (:6
      (bind _returnvalue_7 (Game|SpawnActorfromClass "/Game/CrossyRoad/BluePrints/Road.Road_C" (Math|Transform|MakeTransform SpawnLocation "0, 0, 0" "1.000000,1.000000,1.000000") "Undefined" 0 0))
      (return _returnvalue_7))
    (:7
      (bind _returnvalue_8 (Game|SpawnActorfromClass "/Game/CrossyRoad/BluePrints/River.River_C" (Math|Transform|MakeTransform SpawnLocation "0, 0, 0" "1.000000,1.000000,1.000000") "Undefined" 0 0))
      (return _returnvalue_8))
    (:8
      (bind _returnvalue_9 (Game|SpawnActorfromClass "/Game/CrossyRoad/BluePrints/River.River_C" (Math|Transform|MakeTransform SpawnLocation "0, 0, 0" "1.000000,1.000000,1.000000") "Undefined" 0 0))
      (return _returnvalue_9))
    (:9
      (bind _returnvalue_10 (Game|SpawnActorfromClass "/Game/CrossyRoad/BluePrints/RailRoad.RailRoad_C" (Math|Transform|MakeTransform SpawnLocation "0, 0, 0" "1.000000,1.000000,1.000000") "Undefined" 0 0))
      (return _returnvalue_10))))
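; Railroad lane actor for a Crossy Road-style game that periodically sends trains along the track.
; BeginPlay randomly fixes the travel direction from the Start or End marker and starts a looping timer with a randomized interval.
; Each tick of that timer has a coin-flip chance to spawn crossing lights via LightOn, a BP_Train and train audio.
; An unconnected loop for scattering lights along the crossing never runs.
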(event Custom|Spawn%20Vehicles
  (if (Math|Random|RandomBool)
    (if (Variables|Default|GetVehicleSpawnLocation)
      (CallFunction|Lighton)
      (Game|SpawnActorfromClass "/Game/CrossyRoad/BluePrints/BP_Train.BP_Train_C" (Math|Transform|MakeTransform (Variables|Default|GetStartLocation) "0,90.000000, 0" "1.000000,1.000000,1.000000") "Undefined" 0 0)
      (else
        (CallFunction|Lighton)
        (Game|SpawnActorfromClass "/Game/CrossyRoad/BluePrints/BP_Train.BP_Train_C" (Math|Transform|MakeTransform (Variables|Default|GetEndLocation) "0,-90.000000, 0" "1.000000,1.000000,1.000000") "Undefined" 0 0)))
    (Audio|PlaySoundatLocation "/Game/CrossyRoad/Audio/TrainAudio.TrainAudio" (Transformation|GetActorLocation) "0, 0, 0" 1.0 1.0 0.0 0 0 0 0)))

(event EventBeginPlay
  (Variables|Default|SetStartLocation (Transformation|GetWorldLocation (Variables|Default|GetStart)))
  (Variables|Default|SetEndLocation (Transformation|GetWorldLocation (Variables|Default|GetEnd)))
  (Variables|Default|SetVehicleSpawnLocation (Math|Random|RandomBool))
  (Utilities|Time|SetTimerbyEvent (delegate Custom|Spawn%20Vehicles) (Math|Random|RandomFloatinRange 8.0 1e+01) true))

(event Collision|EventActorBeginOverlap
  (params (OtherActor :type Actor%20Object%20Reference))
  (|CallParentFunction OtherActor) ; This node is disabled and will not be called.\nDrag off pins to build functionality.
)

(event EventTick
  (params (DeltaSeconds :type Float%20%28single-precision%29))
  (|CallParentFunction DeltaSeconds) ; This node is disabled and will not be called.\nDrag off pins to build functionality.
)

(fn ConstructionScript
  (|CallParentFunction))

(fn Lighton
  (Variables|Default|SetTrainLights (Transformation|GetWorldLocation (Variables|Default|GetCrossing)))
  (Game|SpawnActorfromClass "/Game/CrossyRoad/BluePrints/unused/TrainLights.TrainLights_C" (Math|Transform|MakeTransform (Variables|Default|GetTrainLights) "0, 0, 0" "1.000000,1.000000,1.000000") "Undefined" 0 0))
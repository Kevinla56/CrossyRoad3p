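; Road actor for a Crossy Road-style game that spawns vehicle traffic from one of its two ends.
; On BeginPlay it caches the Start and End world locations and randomly picks one end as the spawn side for its lifetime.
; A looping timer, with its interval randomized once, flips a coin each tick to spawn a BP_Vehicle there, rotated according to that side.
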(event Custom|Spawn%20Vehicles
  (if (Math|Random|RandomBool)
    (if (Variables|Default|GetVehicleSpawnLocation)
      (Game|SpawnActorfromClass "/Game/CrossyRoad/BluePrints/BP_Vehicle.BP_Vehicle_C" (Math|Transform|MakeTransform (Variables|Default|GetStartLocation) "0,90.000000, 0" "1.000000,1.000000,1.000000") "Undefined" 0 0)
      (else
        (Game|SpawnActorfromClass "/Game/CrossyRoad/BluePrints/BP_Vehicle.BP_Vehicle_C" (Math|Transform|MakeTransform (Variables|Default|GetEndLocation) "0,-90.000000, 0" "1.000000,1.000000,1.000000") "Undefined" 0 0)))))

(event EventBeginPlay
  (Variables|Default|SetStartLocation (Transformation|GetWorldLocation (Variables|Default|GetStart)))
  (Variables|Default|SetEndLocation (Transformation|GetWorldLocation (Variables|Default|GetEnd)))
  (Variables|Default|SetVehicleSpawnLocation (Math|Random|RandomBool))
  (Utilities|Time|SetTimerbyEvent (delegate Custom|Spawn%20Vehicles) (Math|Random|RandomFloatinRange 2.0 3.0) true))

(event Collision|EventActorBeginOverlap
  (params (OtherActor :type Actor%20Object%20Reference))
  (|CallParentFunction OtherActor) ; This node is disabled and will not be called.\nDrag off pins to build functionality.
)

(event EventTick
  (params (DeltaSeconds :type Float%20%28single-precision%29))
  (|CallParentFunction DeltaSeconds) ; This node is disabled and will not be called.\nDrag off pins to build functionality.
)

(fn ConstructionScript
  (|CallParentFunction))
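; TrainLights is a railway crossing warning signal for the CrossyRoad game, stored in an unused folder.
; On BeginPlay it plays the crossing audio at its location and alternates visibility between the left and right lights at one-second intervals.
; The blink is a fixed, unrolled chain of delays that runs two full left-right cycles once, then leaves both lights off.
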(event EventBeginPlay
  (bind _left_light (Variables|Default|GetLeft%20Light))
  (bind _left_light_2 (Variables|Default|GetLeft%20Light))
  (bind _right_light (Variables|Default|GetRight%20Light))
  (bind _right_light_2 (Variables|Default|GetRight%20Light))
  (Audio|PlaySoundatLocation "/Game/CrossyRoad/Audio/CrossingAudio.CrossingAudio" (Transformation|GetActorLocation) "0, 0, 0" 1.0 1.0 0.0 0 0 0 0)
  (Rendering|SetVisibility _left_light_2 true false)
  (Utilities|FlowControl|Delay 1.0)
  (Rendering|SetVisibility _left_light_2 false false)
  (Rendering|SetVisibility _right_light true false)
  (Utilities|FlowControl|Delay 1.0)
  (Rendering|SetVisibility _right_light false false)
  (Rendering|SetVisibility _left_light true false)
  (Utilities|FlowControl|Delay 1.0)
  (Rendering|SetVisibility _left_light false false)
  (Rendering|SetVisibility _right_light_2 true false)
  (Utilities|FlowControl|Delay 1.0)
  (Rendering|SetVisibility _right_light_2 false false))

(fn ConstructionScript)
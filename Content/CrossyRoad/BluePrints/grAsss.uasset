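; A Crossy Road level-piece Blueprint, apparently a grass strip, that scatters environment spawners and trees when play begins.
; It steps along Y from the Start component, with the step count derived from the distance to End, and randomly places EnvironmentSpawner actors at about one in five steps.
; Each successful roll also spawns a BP_Tree at both fixed TreeBarrier markers, so those trees can stack or be absent entirely.
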(event EventBeginPlay
  (Variables|Default|SetStartLocation (Transformation|GetWorldLocation (Variables|Default|GetStart)))
  (Variables|Default|SetEndLocation (Transformation|GetWorldLocation (Variables|Default|GetEnd)))
  (for _index (range 0 (Math|Float|Truncate (/ (Math|Vector|Distance(Vector) (Variables|Default|GetStartLocation) (Variables|Default|GetEndLocation)) 85.0)))
    (if (> (Math|Random|RandomFloat) 0.8)
      (Game|SpawnActorfromClass "/Game/CrossyRoad/BluePrints/EnvironmentSpawner.EnvironmentSpawner_C" (Math|Transform|MakeTransform (Math|Vector|MakeVector (.x (Variables|Default|GetStartLocation)) (+ (* _index 90) (.Y (Math|Vector|BreakVector (Variables|Default|GetStartLocation)))) (.z (Variables|Default|GetStartLocation))) "0, 0, 0" "1.000000,1.000000,1.000000") "Undefined" 0 0)
      (Variables|Default|SetTreeBarr (Transformation|GetWorldLocation (Variables|Default|GetTreeBarrier1)))
      (Variables|Default|SetTreeBarr1 (Transformation|GetWorldLocation (Variables|Default|GetTreeBarrier)))
      (Game|SpawnActorfromClass "/Game/CrossyRoad/BluePrints/BP_Tree.BP_Tree_C" (Math|Transform|MakeTransform (Variables|Default|GetTreeBarr1) "0, 0, 0" "1.000000,1.000000,1.000000") "Undefined" 0 0)
      (Game|SpawnActorfromClass "/Game/CrossyRoad/BluePrints/BP_Tree.BP_Tree_C" (Math|Transform|MakeTransform (Variables|Default|GetTreeBarr) "0, 0, 0" "1.000000,1.000000,1.000000") "Undefined" 0 0))))

(fn ConstructionScript
  (|CallParentFunction))
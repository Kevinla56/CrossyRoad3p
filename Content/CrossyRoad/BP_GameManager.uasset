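; BP_GameManager tracks the player's step count in the Crossy Road game and owns the HUD.
; On BeginPlay it creates WBP_HUD, adds it to the viewport, passes itself in as GameManager and caches the widget.
; IncrementSteps adds one to Steps, then calls the HUD's StepCounterFunc directly, so the counter is notified on each step.
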(event EventBeginPlay
  (bind _returnvalue (UserInterface|CreateWidget "/Game/CrossyRoad/UI/WBP_HUD.WBP_HUD_C"))
  (UserInterface|Viewport|AddtoViewport _returnvalue 0)
  (Variables|/Game/CrossyRoad/UI/WBP_HUD.WBP_HUD_C|SetGameManager _returnvalue self)
  (Variables|Default|SetHUD%20Widget _returnvalue))

(fn ConstructionScript)

(fn IncrementSteps
  (Variables|Default|SetSteps (+ (Variables|Default|GetSteps) 1))
  (Default|StepCounterFunc (Variables|Default|GetHUD%20Widget)))